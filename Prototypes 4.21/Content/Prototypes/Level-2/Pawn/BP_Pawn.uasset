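; BP_Pawn is a prototype enemy that chases and attacks the player's CombatCharacter, tracking idle, moving, attacking, damaged and dead states with booleans.
; PawnSensing triggers AIMoveTo, while Tick checks Radius overlap to attack and applies damage once IsAttackFinished is set.
; Damaged reduces health and, on death, plays Death and notifies a Health object, with which SetHealth registers the enemy.
; Dead destroys the actor.
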(event `self.ReceiveBeginPlay`
  (set `self.isIdle` true)
  (set `self.isAttacking` false)
  (set `self.isDamaged` false)
  (set `self.isMoving` false)
  (set `self.isDead` false))

(event `self.ReceiveTick`
  (params (DeltaSeconds :type "Float (single-precision)"))
  (`self.Tick_Fight`)
  (`self.Damage Player`))

(event `Tick_Fight`
  ;[1 1 1] Idle <--> Fight
  (if (`self.isDead`)
    _
    (elif (`PrimitiveComponent.IsOverlappingActor` (`self.Radius`) (`GameplayStatics.GetPlayerPawn` 0))
      (set `self.isIdle` false)
      (set `self.isAttacking` true)
      (set `self.isMoving` false)
      (elif (not (`self.isMoving`))
        (set `self.isAttacking` false)
        (set `self.isIdle` true)))))

(event `self.PawnSensing.OnSeePawn`
  (params (Pawn :type "Pawn Object Reference"))
  ;[1 1 1] Move to Player
  (if (`self.isDead`)
    _
    (elif (`PrimitiveComponent.IsOverlappingActor` (`self.Radius`) (`GameplayStatics.GetPlayerPawn` 0))
      (set `self.isMoving` false)
      (set `self.isAttacking` true)
      (else
        (bind _ascombat_character (cast `/Game/FirstPersonBP/Blueprints/CombatCharacter` Pawn))
        (`|AIMoveTo` self (0.0 0.0 0.0) _ascombat_character (`self.acceptanceRadius`)
          (:`then`
            (set `self.isMoving` true)
            (set `self.isIdle` false)
            (set `self.isAttacking` false)))))))

(event `Damage Player`
  ;[1 1 1] Deal Damage
  (if (`self.isAttacking`)
    (if (`self.isAttackFinished`)
      (set `self.isAttacking` false)
      (bind _ascombat_character (cast `/Game/FirstPersonBP/Blueprints/CombatCharacter` (`GameplayStatics.GetPlayerPawn` 0)))
      (`/Game/FirstPersonBP/Blueprints/CombatCharacter.Damaged` _ascombat_character (`self.dmgOutput`))
      (`/Engine/EditorBlueprintResources/StandardMacros.DoOnce` false :!label _label
        (:`Completed`
          (`AudioComponent.Play` (`self.Jab`) 0.0)
          (bind _asanim_bp_pawn (cast `/Game/Prototypes/Level-2/Pawn/AnimBP_Pawn` (`SkeletalMeshComponent.GetAnimInstance` (`self.Mesh`))))
          (`/Game/Prototypes/Level-2/Pawn/AnimBP_Pawn.AnimNotify_StopHit` _asanim_bp_pawn)
          (goto _label :!via `Reset`))))))

(event `Damaged`
  (params (dmg :type "Float (double-precision)"))
  (bind _returnvalue (- (`self.currentHealth`) dmg))
  (bind _output_get (set `self.currentHealth` _returnvalue))
  (`KismetSystemLibrary.PrintString` (`KismetStringLibrary.Conv_DoubleToString` _output_get))
  (if (<= _returnvalue 0.0)
    (set `self.isDead` true)
    (set `self.currentHealth` 0.0)
    (`AudioComponent.Play` (`self.Death`) 0.0)
    (bind _ashealth (cast `/Game/Prototypes/Level-2/Blueprints/Health` (`self.Health`)))
    (`/Game/Prototypes/Level-2/Blueprints/Health.EpicaVictoriaRoyal` _ashealth)
    (else
      (set `self.isDamaged` true))))

(event `Dead`
  (`self.K2_DestroyActor`))

(fn `SetHealth`
  (params (NewParam :type "/Game/Prototypes/Level-2/Blueprints/Health Object Reference"))
  (bind _output_get (set `self.Health` NewParam))
  (`/Game/Prototypes/Level-2/Blueprints/Health.AddEnemy` _output_get self))

(fn `UserConstructionScript`)