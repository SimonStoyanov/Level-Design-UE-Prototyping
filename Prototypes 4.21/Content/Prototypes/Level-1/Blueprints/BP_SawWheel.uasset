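; BP_SawWheel is a saw hazard that travels along a spline and kills the first-person player.
; On BeginPlay the MoveSaw timeline drives SawMesh along the spline, with distance set by track value, spline length and Speed.
; Any actor overlap calls Death on player pawn 0 if it is a FirstPersonCharacter, without checking which actor overlapped.
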(event `self.ReceiveBeginPlay`
  (bind _spline (`self.Spline`))
  (bind (_direction _newtrack_0) (`Timeline|MoveSaw`)
    (:`Update`
      (`SceneComponent.K2_SetWorldLocation` (`self.SawMesh`) (`SplineComponent.GetLocationAtDistanceAlongSpline` _spline (* _newtrack_0 (`SplineComponent.GetSplineLength` _spline) (`self.Speed`)) "World") false false))))

(event `self.ReceiveActorBeginOverlap`
  (params (OtherActor :type "Actor Object Reference"))
  (bind _asfirst_person_character (cast `/Game/FirstPersonBP/Blueprints/FirstPersonCharacter` (`GameplayStatics.GetPlayerPawn` OtherActor)))
  (`/Game/FirstPersonBP/Blueprints/FirstPersonCharacter.Death` _asfirst_person_character))

(fn `UserConstructionScript`)