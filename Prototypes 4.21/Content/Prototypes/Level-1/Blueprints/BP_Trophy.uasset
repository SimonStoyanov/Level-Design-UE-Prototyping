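; BP_Trophy is a prototype win pickup that spins a fixed amount on all axes every tick.
; A begin overlap on TrophyCol prints an interact prompt through a DoOnce when it comes from a sweep, otherwise resetting it.
; Pressing E while the player overlaps destroys the actor first, then prints win messages and plays a timeline.
; That timeline's Update requests a 1Corridor level instance at the origin as the intended restart.
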(event `self.ReceiveTick`
  (params (DeltaSeconds :type "Float (single-precision)"))
  (`SceneComponent.K2_AddLocalRotation` (`self.StaticMeshComponent`) (struct :`Pitch` 60.0 :`Yaw` 60.0 :`Roll` 60.0) false false))

(event `self.TrophyCol.OnComponentBeginOverlap`
  (params (OverlappedComponent :type "PrimitiveComponent Object Reference") (OtherActor :type "Actor Object Reference") (OtherComp :type "PrimitiveComponent Object Reference") (OtherBodyIndex :type Integer) (bFromSweep :type Boolean) (SweepResult :type "HitResult Structure (by ref)"))
  (if bFromSweep
    (`/Engine/EditorBlueprintResources/StandardMacros.DoOnce` false :!label _label
      (:`Completed`
        (`KismetSystemLibrary.PrintString` "Press E to Interact")))
    (else
      (goto _label :!via `Reset`))))

(event `Key|E`
  (params (Key :type "Key Structure"))
  (:`Pressed`
    (if (`PrimitiveComponent.IsOverlappingActor` (`self.TrophyCol`) (`GameplayStatics.GetPlayerPawn` (stale `self.TrophyCol.OnComponentBeginOverlap` OtherActor)))
      (`self.K2_DestroyActor`)
      (`KismetSystemLibrary.PrintString` "You Win!")
      (`KismetSystemLibrary.PrintString` "Restarting Game...")
      (`Timeline|Timeline_0` :`NewTime` 1.0
        (:`Update`
          (`LevelStreamingDynamic.LoadLevelInstanceBySoftObjectPtr` "/Game/Prototypes/Level-1/1-Corridor.1-Corridor"))))))

(fn `UserConstructionScript`)